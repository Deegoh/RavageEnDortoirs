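; Enemy AI character that patrols waypoints, turns suspicious, chases the player and fires projectiles.
; A detection box flags suspicion, making the eyes track the player while patrolling.
; Each tick, a forward eye trace refreshes a detection countdown, which selects Attack or Chase by distance, otherwise Suspicious or Patrol.
; Each mode blends walk speed and recolors a dynamic material, with a Delay on Tick pacing shots while the player is in view.
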(event OnComponentBeginOverlap(DetectionArea)
  (params (OverlappedComponent :type Primitive%20Component%20Object%20Reference) (OtherActor :type Actor%20Object%20Reference) (OtherComp :type Primitive%20Component%20Object%20Reference) (OtherBodyIndex :type Integer) (bFromSweep :type Boolean) (SweepResult :type Hit%20Result%20Structure%20%28by%20ref%29))
  ;[1 1 1] Detection Precess
  (bind _asmy_character (Utilities|Casting|CastToMyCharacter OtherActor))
  (if (Variables|/Game/Blueprints/MyCharacter.MyCharacter_C|GetIsDead _asmy_character)
    (Variables|Default|SetIsSupecious false)
    (else
      (Variables|Default|SetIsSupecious true))))

(event OnComponentEndOverlap(DetectionArea)
  (params (OverlappedComponent :type Primitive%20Component%20Object%20Reference) (OtherActor :type Actor%20Object%20Reference) (OtherComp :type Primitive%20Component%20Object%20Reference) (OtherBodyIndex :type Integer))
  ;[1 1 1] Detection Precess
  (Utilities|Casting|CastToMyCharacter OtherActor)
  (Variables|Default|SetIsSupecious false))

(event Collision|EventHit
  (params (MyComp :type Primitive%20Component%20Object%20Reference) (Other :type Actor%20Object%20Reference) (OtherComp :type Primitive%20Component%20Object%20Reference) (bSelfMoved :type Boolean) (HitLocation :type Vector :default "0, 0, 0") (HitNormal :type Vector :default "0, 0, 0") (NormalImpulse :type Vector) (Hit :type Hit%20Result%20Structure%20%28by%20ref%29))
  (bind _returnvalue (Math|Vector|VectorLength NormalImpulse))
  (bind _returnvalue_2 (>= _returnvalue 0.0))
  (Physics|SetSimulatePhysics (Variables|Collision|GetCapsuleComponent) _returnvalue_2)
  (Physics|SetSimulatePhysics (Variables|Character|GetMesh) _returnvalue_2))

(event EventTick
  (params (DeltaSeconds :type Float%20%28single-precision%29))
  ;[1 1 1] Tick
  (Utilities|FlowControl|Sequence
    (:then_0
      ;[1 1 1] Detection Precess
      (CallFunction|EyesTrace))
    (:then_1
      ;[1 1 1] Define AlertMode
      (Math|Float|CompareFloat (Variables|Default|GetDetectionDelayTemp) 0.0
        (:>
          (Variables|Default|SetDetectionDelayTemp (- (Variables|Default|GetDetectionDelayTemp) (Utilities|Time|GetWorldDeltaSeconds)))
          (bind _distance (CallFunction|GetDistancetoPlayer))
          (Math|Float|CompareFloat _distance (Variables|Default|GetAttackDistance)
            (:>
              (Variables|Default|SetAlertMode "NewEnumerator1"))
            (:==
              (Variables|Default|SetAlertMode "NewEnumerator0" :!label _label))
            (:<
              (goto _label))))
        (:==
          (if (Variables|Default|GetIsSupecious) :!label _label_2
            (Variables|Default|SetAlertMode "NewEnumerator2")
            (else
              (Variables|Default|SetAlertMode "NewEnumerator3"))))
        (:<
          (goto _label_2))))
    (:then_2
      ;[1 1 1] Switch On Alert Mode
      (switch Utilities|FlowControl|Switch|SwitchonAlertMode (Variables|Default|GetAlertMode)
        (:NewEnumerator0
          (CallFunction|ChangeSpeed (Variables|Default|GetAttackSpeed))
          (CallFunction|ChangeColor "(R=1.000000,G=0.000000,B=0.000000,A=1.000000)")
          (CallFunction|LookforSuspect)
          (CallFunction|Chase)
          (Utilities|FlowControl|Delay (Variables|Default|GetFireRate))
          (if (Variables|Default|GetIsInView)
            (CallFunction|Attack)))
        (:NewEnumerator1
          (CallFunction|ChangeSpeed (Variables|Default|GetChaseSpeed))
          (CallFunction|ChangeColor "(R=1.000000,G=0.000000,B=0.000000,A=1.000000)")
          (CallFunction|LookforSuspect)
          (CallFunction|Chase))
        (:NewEnumerator2
          (CallFunction|ChangeSpeed (Variables|Default|GetSuspeciousSpeed))
          (CallFunction|ChangeColor "(R=1.000000,G=0.075480,B=0.000000,A=1.000000)")
          (CallFunction|LookforSuspect)
          (CallFunction|Patrol :!label _label_3))
        (:NewEnumerator3
          (CallFunction|ChangeSpeed (Variables|Default|GetPatrolSpeed))
          (CallFunction|ChangeColor "(R=0.075141,G=0.805000,B=0.000000,A=1.000000)")
          (CallFunction|ResetEyesRotation)
          (goto _label_3))))))

(event EventBeginPlay
  ;[1 1 1] BeginPlay (Debug Settings)
  (if (Variables|Default|GetDebug)
    (Development|SetHiddeninGame (Variables|Default|GetDetectionArea) false false)
    (Variables|Default|SetTraceDebug "ForOneFrame")))

(fn ConstructionScript
  (bind _detectionarea (Variables|Default|GetDetectionArea))
  (Transformation|SetRelativeLocation _detectionarea (Variables|Default|GetDetectionAreaLocation) false false)
  (Components|Box|SetBoxExtent _detectionarea (Variables|Default|GetDetectionAreaSize) true)
  (bind _returnvalue (Rendering|Material|CreateDynamicMaterialInstance (Variables|Character|GetMesh) 0 "/Game/Materials/Enemy_Material.Enemy_Material" :!class /Script/Engine.PrimitiveComponent))
  (Variables|Default|SetMaterialInstance _returnvalue))

(fn Patrol
  (if (<= (Transformation|GetDistanceTo (Utilities|Array|Get(acopy) (Variables|Default|GetWayPoints) (Variables|Default|GetCurrentPoint))) 2e+02)
    (if (>= (Variables|Default|GetCurrentPoint) (Utilities|Array|Length (Variables|Default|GetWayPoints)))
      (Variables|Default|SetCurrentPoint 0)
      (else
        (Variables|Default|SetCurrentPoint (+ (Variables|Default|GetCurrentPoint) 1))))
    (else
      (AI|Navigation|SimpleMovetoActor (Pawn|GetController) (Utilities|Array|Get(acopy) (Variables|Default|GetWayPoints) (Variables|Default|GetCurrentPoint))))))

(fn Chase
  (AI|Navigation|SimpleMovetoActor (Pawn|GetController) (Game|Player|GetPlayerPawn 0)))

(fn Attack
  (bind _shooter (Variables|Default|GetShooter))
  (Game|SpawnActorfromClass "/Game/Blueprints/Projectile.Projectile_C" (Math|Transform|MakeTransform (Transformation|GetWorldLocation _shooter) (Transformation|GetWorldRotation _shooter)) "AlwaysSpawn" 0 0))

(fn LookforSuspect
  (bind _eyes (Variables|Default|GetEyes))
  (Transformation|SetWorldRotation _eyes (Math|Rotator|FindLookatRotation (Transformation|GetWorldLocation _eyes) (Transformation|GetActorLocation (Game|Player|GetPlayerPawn 0))) true false))

(fn ResetEyesRotation
  (Transformation|SetRelativeRotation (Variables|Default|GetEyes) "0, 0, 0" true false))

(fn ChangeColor
  (params (NewColor :type Linear%20Color%20Structure))
  (bind _materialinstance (Variables|Default|GetMaterialInstance))
  (Rendering|Material|SetVectorParameterValue _materialinstance "Color" NewColor :!class /Script/Engine.MaterialInstanceDynamic)
  (Rendering|Material|SetMaterial (Variables|Character|GetMesh) 0 _materialinstance))

(fn ChangeSpeed
  (params (NewSpeed :type Float%20%28single-precision%29))
  (Variables|/Script/Engine.CharacterMovementComponent|SetMaxWalkSpeed (Variables|Character|GetCharacterMovement) (Math|Float|Lerp NewSpeed (Variables|/Script/Engine.CharacterMovementComponent|GetMaxWalkSpeed (Variables|Character|GetCharacterMovement)) 0.85)))

(fn GetDistancetoPlayer
  (return (Transformation|GetDistanceTo (Game|Player|GetPlayerPawn 0))))

(fn EyesTrace
  (bind _eyes (Variables|Default|GetEyes))
  (bind _returnvalue (Transformation|GetWorldLocation _eyes))
  (bind _outhit (Collision|LineTraceByChannel _returnvalue (+ _returnvalue (* (Math|Vector|GetForwardVector _eyes) (Variables|Default|GetFieldOfView))) "TraceTypeQuery1" false 0 (Variables|Default|GetTraceDebug)))
  (bind _asmy_character (Utilities|Casting|CastToMyCharacter (.HitActor (Collision|BreakHitResult _outhit)))
    (:then
      (if (Variables|/Game/Blueprints/MyCharacter.MyCharacter_C|GetIsDead _asmy_character)
        (Variables|Default|SetDetectionDelayTemp 0.0)
        (else
          (Variables|Default|SetIsInView true)
          (Variables|Default|SetDetectionDelayTemp (Variables|Default|GetDetectionDelay)))))
    (:CastFailed
      (Variables|Default|SetIsInView false))))