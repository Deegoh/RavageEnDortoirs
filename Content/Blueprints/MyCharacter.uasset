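; MyCharacter is a character Blueprint with simple health and death handling.
; BeginPlay resets health to full and clears the dead flag.
; AnyDamage subtracts incoming damage, and at zero or below clamps health, sets the dead flag, disables input through player controller 0, and hides the mesh with its children.
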(event EventAnyDamage
  (params (Damage :type Float%20%28single-precision%29) (DamageType :type Damage%20Type%20Object%20Reference) (InstigatedBy :type Controller%20Object%20Reference) (DamageCauser :type Actor%20Object%20Reference))
  ;[1 1 1] Damage / Death
  (Variables|Default|SetHealth (- (Variables|Default|GetHealth) Damage))
  (if (<= (Variables|Default|GetHealth) 0.0)
    (Variables|Default|SetHealth 0.0)
    (Variables|Default|SetIsDead true)
    (Input|DisableInput (Game|GetPlayerController 0))
    (Rendering|SetVisibility (Variables|Character|GetMesh) false true)))

(event EventBeginPlay
  ;[1 1 1] Begin Play
  (Variables|Default|SetHealth 1e+02)
  (Variables|Default|SetIsDead false))

(fn ConstructionScript)